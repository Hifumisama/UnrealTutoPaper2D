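; Enemy actor that fires projectiles while the hero is within its detection sphere and destroys itself when its life points run out.
; Sphere overlaps with HeroCharacter toggle a detection flag, which Tick reads to spawn an EnnemyProjectile at the ProjectileSpawner after a delay.
; LoseHP subtracts incoming damage from life points.
; An animation function picks Jump when falling, otherwise always Run, as its hardcoded branch ignores IsMoving.
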(event `self.ReceiveBeginPlay`)

(event `self.ReceiveTick`
  (params (DeltaSeconds :type "Float (single-precision)"))
  ;[1 1 1] Tire un projectile
  (if (`self.DetectedCharacter`)
    (`KismetSystemLibrary.Delay` 2.0)
    (if true
      (`|SpawnActorFromClass` "/Game/Blueprint/EnnemyProjectile.EnnemyProjectile_C" (`SceneComponent.K2_GetComponentToWorld` (`self.projectileSpawner`)) "Undefined" "OverrideRootScale" null null))))

(event `LoseHP`
  (params (Damage :type Integer))
  ;[1 1 1] Gère la detection et l'application des dommages
  (bind _output_get (set `self.LifePoints` (- (`self.LifePoints`) Damage)))
  (if (<= _output_get 0)
    (`self.K2_DestroyActor`)))

(event `self.Sphere.OnComponentBeginOverlap`
  (params (OverlappedComponent :type "PrimitiveComponent Object Reference") (OtherActor :type "Actor Object Reference") (OtherComp :type "PrimitiveComponent Object Reference") (OtherBodyIndex :type Integer) (bFromSweep :type Boolean) (SweepResult :type "HitResult Structure (by ref)"))
  ;[1 1 1] octroie la détection du héros pour notre ennemi
  (cast `/Game/Blueprint/Character/HeroCharacter` OtherActor)
  (set `self.DetectedCharacter` true))

(event `self.Sphere.OnComponentEndOverlap`
  (params (OverlappedComponent :type "PrimitiveComponent Object Reference") (OtherActor :type "Actor Object Reference") (OtherComp :type "PrimitiveComponent Object Reference") (OtherBodyIndex :type Integer))
  ;[1 1 1] octroie la détection du héros pour notre ennemi
  (cast `/Game/Blueprint/Character/HeroCharacter` OtherActor)
  (set `self.DetectedCharacter` false))

(fn `AnimationStateMachine`
  (params (IsFalling :type Boolean) (IsMoving :type Boolean))
  (returns (NewParam2 :type "PaperFlipbook Object Reference"))
  (locals (AnimationState :type "/Game/Data/AnimationState Enum"))
  (if IsFalling
    (set `local.AnimationState` "NewEnumerator2")
    (elif true
      (set `local.AnimationState` "NewEnumerator1")
      (else
        (set `local.AnimationState` "NewEnumerator0"))))
  (return (select `/Game/Data/AnimationState` (`local.AnimationState`) :`NewEnumerator0` (`self.Idle`) :`NewEnumerator1` (`self.Run`) :`NewEnumerator2` (`self.Jumping`))))

(fn `UserConstructionScript`)