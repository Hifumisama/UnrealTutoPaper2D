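; PickUpHPMax is a pickup that permanently raises the player's maximum HP through saved data.
; On any actor overlap it runs the parent overlap logic, then adds Modify to MaxHP in the PlayerStats of DataToChange.
; It passes the updated struct to the DataManagementSystem object to save, then immediately calls LoadData.
; The overlapping actor is not checked here.
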(event `self.ReceiveActorBeginOverlap`
  (params (OtherActor :type "Actor Object Reference"))
  (bind _datatochange_playerstats (break `/Game/Data/SaveGameData/PlayerData` (`self.DataToChange`)))
  (bind _datamanagementsystemobject (`self.DataManagementSystemObject`))
  (`parent.ReceiveActorBeginOverlap` OtherActor)
  (bind _structout (setmembers `/Game/Data/SaveGameData/CharacterStats` :`StructRef` (make `/Game/Data/SaveGameData/CharacterStats` "Shara" 1 (+ (`.MaxHP_17_33E0DCF24DF566C3ECEDB9994CA89EE2` (break `/Game/Data/SaveGameData/CharacterStats` _datatochange_playerstats)) (`self.Modify`)))))
  (bind _output_get (set `self.DataToChange` (make `/Game/Data/SaveGameData/PlayerData` _structout)))
  (`/Game/Data/DatamanagementSystem.SaveData` _datamanagementsystemobject _output_get)
  (`/Game/Data/DatamanagementSystem.LoadData` _datamanagementsystemobject))

(fn `UserConstructionScript`
  (`parent.UserConstructionScript`))