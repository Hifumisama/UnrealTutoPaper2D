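; Generic pickup actor that changes one entry in the player's data when a HeroCharacter overlaps its box.
; ValueType selects whether the entry named by VariableToChange gets a replacement string or has its integer raised by IncrementValue.
; The updated map is written back into the player data struct, which the character saves and reloads before the pickup destroys itself.
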(event `self.Box.OnComponentBeginOverlap`
  (params (OverlappedComponent :type "PrimitiveComponent Object Reference") (OtherActor :type "Actor Object Reference") (OtherComp :type "PrimitiveComponent Object Reference") (OtherBodyIndex :type Integer) (bFromSweep :type Boolean) (SweepResult :type "HitResult Structure (by ref)"))
  (bind _variabletochange (`self.VariableToChange`))
  (bind _ashero_character (cast `/Game/Blueprint/Character/HeroCharacter` OtherActor))
  (bind _output_get (set `self.HeroCharacter` _ashero_character))
  (bind _output_get_2 (set `self.DataToChange` (`/Game/Blueprint/Character/HeroCharacter.LocalPlayerData` _output_get)))
  (set `self.StringMap` (break `/Game/Data/SaveGameData/PlayerDataMaps` _output_get_2))
  (set `self.IntMap` (`.PlayerInt_10_54CE1D614CF3290B3B224585624C1191` (break `/Game/Data/SaveGameData/PlayerDataMaps` _output_get_2)))
  (switch `/Game/Data/SaveGameData/ValueTypeSelector` (`self.ValueType`)
    (:`NewEnumerator1`
      (`self.UpdateString` (`self.StringMap`) _variabletochange))
    (:`NewEnumerator2`
      (`self.UpdateInt` (`self.IntMap`) _variabletochange)))
  (`/Game/Blueprint/Character/HeroCharacter.SaveData` (`self.HeroCharacter`) (`self.DataToChange`))
  (`/Game/Blueprint/Character/HeroCharacter.LoadData` (`self.HeroCharacter`))
  (`self.K2_DestroyActor`))

(fn `UpdateInt`
  (params (TargetMap :type "Map of /Game/Data/SaveGameData/PlayerStatEnum Enum to Integer (by ref)" :default _) (Key :type "/Game/Data/SaveGameData/PlayerStatEnum Enum (by ref)" :default "NewEnumerator0"))
  (bind _datatochange_playerstring (break `/Game/Data/SaveGameData/PlayerDataMaps` (`self.DataToChange`)))
  (`BlueprintMapLibrary.Map_Add` TargetMap Key (+ (`BlueprintMapLibrary.Map_Find` TargetMap Key) (`self.IncrementValue`)))
  (bind _structout (setmembers `/Game/Data/SaveGameData/PlayerDataMaps` :`StructRef` (make `/Game/Data/SaveGameData/PlayerDataMaps` _datatochange_playerstring (`local.TargetMap`))))
  (set `self.DataToChange` _structout))

(fn `UpdateString`
  (params (StringMap :type "Map of /Game/Data/SaveGameData/PlayerStatEnum Enum to String" :default _) (VariableToChange :type "/Game/Data/SaveGameData/PlayerStatEnum Enum" :default "NewEnumerator0"))
  (bind (_datatochange_playerstring _datatochange_playerint) (break `/Game/Data/SaveGameData/PlayerDataMaps` (`self.DataToChange`)))
  (`BlueprintMapLibrary.Map_Add` StringMap VariableToChange (`self.StringToReplace`))
  (bind _structout (setmembers `/Game/Data/SaveGameData/PlayerDataMaps` :`StructRef` (make `/Game/Data/SaveGameData/PlayerDataMaps` (`local.StringMap`) _datatochange_playerint)))
  (set `self.DataToChange` _structout))

(fn `UserConstructionScript`)