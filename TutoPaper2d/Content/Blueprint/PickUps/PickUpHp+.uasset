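; Health pickup Blueprint that adds HP to the hero when an actor overlaps it.
; The overlap event calls the parent implementation, then adds HpToAdd to ActualHp on the Hero reference, with no clamp.
; Hero is not assigned in this Blueprint, and OtherActor is only passed to the parent call.
; BeginPlay, Tick and the construction script add no logic of their own.
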(event `self.ReceiveActorBeginOverlap`
  (params (OtherActor :type "Actor Object Reference"))
  (bind _hero (`self.Hero`))
  (`parent.ReceiveActorBeginOverlap` OtherActor)
  (set `/Game/Blueprint/Character/HeroCharacter.ActualHp` (+ (`/Game/Blueprint/Character/HeroCharacter.ActualHp` _hero) (`self.HpToAdd`)) _hero))

(fn `UserConstructionScript`
  (`parent.UserConstructionScript`))