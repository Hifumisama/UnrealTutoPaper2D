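; Pickup actor that adds extra lives to the hero when touched.
; When its Box is overlapped by a HeroCharacter, it adds IncrementValue to the LifeCount read from that character's LocalPlayerData.
; It passes a PlayerData struct with the new count to the character's SaveData, prints the character's LifeCount, then destroys itself.
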(event `self.Box.OnComponentBeginOverlap`
  (params (OverlappedComponent :type "PrimitiveComponent Object Reference") (OtherActor :type "Actor Object Reference") (OtherComp :type "PrimitiveComponent Object Reference") (OtherBodyIndex :type Integer) (bFromSweep :type Boolean) (SweepResult :type "HitResult Structure (by ref)"))
  (bind _ashero_character (cast `/Game/Blueprint/Character/HeroCharacter` OtherActor))
  (bind (_playername _playerlevel _experiencepoints _lifecount) (break `/Game/Blueprint/SaveGameData/PlayerData` (`/Game/Blueprint/Character/HeroCharacter.LocalPlayerData` _ashero_character)))
  (bind _output_get (set `self.LifeCountChanged` (+ _lifecount (`self.IncrementValue`))))
  (bind _structout (setmembers `/Game/Blueprint/SaveGameData/PlayerData` :`StructRef` (make `/Game/Blueprint/SaveGameData/PlayerData` "Shara" 1 0 _output_get)))
  (`/Game/Blueprint/Character/HeroCharacter.SaveData` _ashero_character _structout)
  (`KismetSystemLibrary.PrintString` (`KismetStringLibrary.Conv_IntToString` _lifecount))
  (`self.K2_DestroyActor`))

(fn `UserConstructionScript`)