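; BadGuy is an enemy Blueprint with a Paper2D sprite, providing contact damage, projectile firing and health handling.
; Any sprite overlap damages player 0's HeroCharacter, without checking which actor overlapped.
; FireProjectile, when passed a detected flag, waits briefly, then spawns the given projectile class at the given spawner's transform.
; LooseHP subtracts damage and destroys the actor when ActualHP is at or below MaxHP, rather than zero.
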(event `/Game/Blueprint/EnnemyInterface.FireProjectile`
  (params (IsDetected :type Boolean) (ProjectileSpawner :type "ArrowComponent Object Reference") (ProjectileToSpawn :type "/Game/Blueprint/EnnemyProjectile Class Reference"))
  ;[1 1 1] Tire un projectile
  (if IsDetected
    (`KismetSystemLibrary.Delay` 2.0)
    (if true
      (`|SpawnActorFromClass` ProjectileToSpawn (`SceneComponent.K2_GetComponentToWorld` ProjectileSpawner) "Undefined" "OverrideRootScale" null null))))

(event `/Game/Blueprint/EnnemyInterface.LooseHP`
  (params (Damage :type Integer))
  ;[1 1 1] Gère la detection et l'application des dommages
  (bind _output_get (set `self.ActualHP` (- (`self.ActualHP`) Damage)))
  (if (<= _output_get (`self.MaxHP`))
    (`self.K2_DestroyActor`)))

(event `/Game/Blueprint/EnnemyInterface.DamageOnContact`
  (params (Damage :type Integer))
  (bind _ashero_character (cast `/Game/Blueprint/Character/HeroCharacter` (`GameplayStatics.GetPlayerCharacter` 0)))
  (`/Game/Blueprint/Character/HeroCharacter.LoseHP` _ashero_character Damage))

(event `self.PaperSprite.OnComponentBeginOverlap`
  (params (OverlappedComponent :type "PrimitiveComponent Object Reference") (OtherActor :type "Actor Object Reference") (OtherComp :type "PrimitiveComponent Object Reference") (OtherBodyIndex :type Integer) (bFromSweep :type Boolean) (SweepResult :type "HitResult Structure (by ref)"))
  (`/Game/Blueprint/Projectile.DamageOnContact` (`self.ContactDamageAmount`)))

(fn `UserConstructionScript`)