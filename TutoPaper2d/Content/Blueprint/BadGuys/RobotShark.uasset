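; RobotShark is an enemy Blueprint that moves between its starting position and the location of a MovePoint actor.
; On BeginPlay it caches both locations and plays the MoveInterp timeline at a rate set by Speed.
; Each timeline update lerps the actor's location without sweep.
; When the track is near its end or at zero, it sets a fixed 180-degree rotation rather than adding a turn.
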(event `self.ReceiveBeginPlay`
  (bind _returnvalue_location (`KismetMathLibrary.BreakTransform` (`self.GetTransform`)))
  (bind _returnvalue_location_2 (`KismetMathLibrary.BreakTransform` (`self.GetTransform` (`self.MovePoint`))))
  (`parent.ReceiveBeginPlay`)
  (`|ExecutionSequence`
    (:`then_0`
      (set `self.InitialLocation` _returnvalue_location))
    (:`then_1`
      (set `self.FinalLocation` _returnvalue_location_2)
      (`TimelineComponent.SetPlayRate` (`self.MoveInterp`) (`self.Speed`))
      (bind (_direction _newtrack_0) (`Timeline|MoveInterp`)
        (:`Update`
          (bind _output_get (set `self.ActualLocation` (`KismetMathLibrary.VLerp` (`self.InitialLocation`) (`self.FinalLocation`) _newtrack_0)))
          (`self.K2_SetActorLocation` _output_get)
          (if (or (>= _newtrack_0 0.97) (<= _newtrack_0 0.0))
            (`self.K2_SetActorRotation` (struct :`Yaw` 180.0))))))))

(event `self.ReceiveTick`
  (params (DeltaSeconds :type "Float (single-precision)"))
  (`parent.ReceiveTick` DeltaSeconds))

(fn `UserConstructionScript`
  (`parent.UserConstructionScript`))