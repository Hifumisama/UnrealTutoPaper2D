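; Base logic for a 2D flipbook enemy character that takes damage, can fire projectiles and hurts HeroCharacter on capsule overlap.
; Tick steers it toward the MovingTo actor, but the intended back-and-forth patrol only prints a debug string.
; LooseHP handles hit reactions and death, while FireProjectile spawns shots after a delay.
; State flags feed a priority-based flipbook selector, where the always-true Move check blocks Jump and Fire is ignored.
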(event `self.ReceiveTick`
  (params (DeltaSeconds :type "Float (single-precision)"))
  (`self.MoveEnnemy` DeltaSeconds))

(event `self.ReceiveBeginPlay`
  (set `self.ActualHP` (`self.MaxHP`))
  (set `self.IsSpawning?` true)
  (`self.UpdateAnim`)
  (`KismetSystemLibrary.Delay` 0.2)
  (set `self.IsSpawning?` false)
  (`self.UpdateAnim`)
  (set `self.initialLocation` (`self.K2_GetActorLocation`)))

(event `/Game/Blueprint/BadGuys/EnnemyInterface.FireProjectile`
  (params (IsDetected :type Boolean) (ProjectileSpawner :type "ArrowComponent Object Reference") (ProjectileToSpawn :type "/Game/Blueprint/EnnemyProjectile Class Reference"))
  ;[1 1 1] Tire un projectile
  (if IsDetected
    (set `self.IsFiring?` true)
    (`KismetSystemLibrary.Delay` 2.0)
    (set `self.IsFiring?` false)
    (`|SpawnActorFromClass` ProjectileToSpawn (`SceneComponent.K2_GetComponentToWorld` ProjectileSpawner) "Undefined" "OverrideRootScale" null null)))

(event `/Game/Blueprint/BadGuys/EnnemyInterface.LooseHP`
  (params (Damage :type Integer))
  ;[1 1 1] Gère la detection et l'application des dommages
  (bind _output_get (set `self.ActualHP` (- (`self.ActualHP`) Damage)))
  (if (<= _output_get 0)
    (set `self.IsDead?` true)
    (`self.UpdateAnim`)
    (`KismetSystemLibrary.Delay` 0.5)
    (`self.K2_DestroyActor`)
    (else
      (set `self.IsTakingDamage` true)
      (`self.UpdateAnim`)
      (`KismetSystemLibrary.Delay` 0.2)
      (set `self.IsTakingDamage` false)
      (`self.UpdateAnim`))))

(event `/Game/Blueprint/BadGuys/EnnemyInterface.MoveEnnemy`
  (params (DeltaS :type "Float (single-precision)"))
  (bind _deltadistance_x (`KismetMathLibrary.BreakVector` (`self.DeltaDistance`)))
  ;[1 1 1] permet de se déplacer d'un point A a un point B et inversement
  (bind _output_get (set `self.DeltaDistance` (- (`self.K2_GetActorLocation` (`self.MovingTo`)) (`self.K2_GetActorLocation` self))))
  (`self.AddMovementInput` (`KismetMathLibrary.Normal` _output_get) (* DeltaS (`self.EnnemySpeed`)))
  (`self.UpdateAnim`)
  (if (<= _deltadistance_x 0.1)
    (`KismetSystemLibrary.PrintString` "Hello")))

(event `UpdateAnim`
  (bind _returnedflipbook (`self.AnimStateMachine` (`self.IsSpawning?`) (`self.IsDead?`) (`self.IsTakingDamage`) (>= (`KismetMathLibrary.VSize` (`self.GetVelocity`)) 0.0) (`NavMovementComponent.IsFalling` (`self.CharacterMovement`)) (`self.IsFiring?`)))
  (`PaperFlipbookComponent.SetFlipbook` (`self.Sprite`) _returnedflipbook))

(event `self.CapsuleComponent.OnComponentBeginOverlap`
  (params (OverlappedComponent :type "PrimitiveComponent Object Reference") (OtherActor :type "Actor Object Reference") (OtherComp :type "PrimitiveComponent Object Reference") (OtherBodyIndex :type Integer) (bFromSweep :type Boolean) (SweepResult :type "HitResult Structure (by ref)"))
  (bind _ashero_character (cast `/Game/Blueprint/Character/HeroCharacter` OtherActor))
  (`/Game/Blueprint/Character/HeroCharacter.LoseHP` _ashero_character (`self.ContactDamageAmount`)))

(fn `AnimStateMachine`
  (params (Spawning :type "Boolean (by ref)") (Died :type "Boolean (by ref)") (Damaged :type "Boolean (by ref)") (Move :type "Boolean (by ref)") (Fall :type "Boolean (by ref)") (Fire :type "Boolean (by ref)"))
  (returns (ReturnedFlipbook :type "PaperFlipbook Object Reference"))
  (if Spawning
    (set `self.AnimState` "NewEnumerator5")
    (elif Died
      (bind _output_get (set `self.AnimState` "NewEnumerator4"))
      (elif Damaged
        (set `self.AnimState` "NewEnumerator3")
        (elif Move
          (set `self.AnimState` "NewEnumerator1")
          (elif Fall
            (set `self.AnimState` "NewEnumerator2"))))))
  (switch `/Game/Data/AnimationState` _output_get
    (:`NewEnumerator0`
      (set `self.FlipbookToReturn` (`self.Idle`)))
    (:`NewEnumerator1`
      (set `self.FlipbookToReturn` (`self.Move`)))
    (:`NewEnumerator2`
      (set `self.FlipbookToReturn` (`self.Jump_0`)))
    (:`NewEnumerator3`
      (set `self.FlipbookToReturn` (`self.Damaged`)))
    (:`NewEnumerator4`
      (set `self.FlipbookToReturn` (`self.Die`)))
    (:`NewEnumerator5`
      (set `self.FlipbookToReturn` (`self.Spawn`))))
  (return (`self.FlipbookToReturn`)))

(fn `UserConstructionScript`)