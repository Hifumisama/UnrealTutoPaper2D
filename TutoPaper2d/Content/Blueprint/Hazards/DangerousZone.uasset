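; Hazard zone Blueprint that damages or kills the HeroCharacter when it begins overlapping the zone's Box.
; If Damage meets or exceeds the hero's LifePoints, it destroys the hero and calls Respawn on the PaperGameMode.
; Otherwise it calls LoseHP with Damage and launches the hero by BounceVelocity as a knockback, without overriding existing velocity.
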(event `self.Box.OnComponentBeginOverlap`
  (params (OverlappedComponent :type "PrimitiveComponent Object Reference") (OtherActor :type "Actor Object Reference") (OtherComp :type "PrimitiveComponent Object Reference") (OtherBodyIndex :type Integer) (bFromSweep :type Boolean) (SweepResult :type "HitResult Structure (by ref)"))
  (bind _ashero_character (cast `/Game/Blueprint/Character/HeroCharacter` OtherActor))
  (set `self.Herocharacter` _ashero_character)
  ;[1 1 1] On observe si la quantité de dommage n'est pas égale ou supérieure à notre total de pv
  (if (>= (`self.Damage`) (`/Game/Blueprint/Character/HeroCharacter.LifePoints` (`self.Herocharacter`)))
    ;[1 1 1] Si le perso n'a plus de PV, on lance la fonction de respawn
    (bind _aspaper_game_mode (cast `/Game/Blueprint/PaperGameMode` (`GameplayStatics.GetGameMode`)))
    (`self.K2_DestroyActor` (`self.Herocharacter`))
    (`/Game/Blueprint/PaperGameMode.Respawn` _aspaper_game_mode)
    (else
      ;[1 1 1] Si il lui reste encore des PV on lui en fait perdre selon le nombre de damages prévus
      (`/Game/Blueprint/Character/HeroCharacter.LoseHP` (`self.Herocharacter`) (`self.Damage`))
      (`Character.LaunchCharacter` (`self.Herocharacter`) (`self.BounceVelocity`) false false))))

(fn `UserConstructionScript`)