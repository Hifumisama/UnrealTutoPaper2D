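; Moving platform actor that shuttles back and forth between its starting transform and the transform of a referenced target actor, MovingTo.
; BeginPlay caches both endpoints, and Tick calls IncrementLerp or DecrementLerp depending on a direction flag.
; Each function advances an alpha by delta time times Speed, applies a linearly interpolated transform without sweep, then flips direction on reaching the end.
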(event `self.ReceiveBeginPlay`
  (set `self.initialLocation` (`self.GetTransform`))
  (set `self.FinalLocation` (`self.GetTransform` (`self.MovingTo`))))

(event `self.ReceiveTick`
  (params (DeltaSeconds :type "Float (single-precision)"))
  (set `self.DeltaS` DeltaSeconds)
  (if (`self.ChangeDirection`)
    (`self.DecrementLerp`)
    (else
      (`self.IncrementLerp`))))

(fn `DecrementLerp`
  ;[1 1 1] On calcule la vitesse de déplacement de l'objet suivant le framerate, la vitesse, et on la set à notre Alpha de déplacement
  (bind _output_get (set `self.Translation` (- (`self.Translation`) (* (`self.DeltaS`) (`self.Speed`)))))
  (`self.K2_SetActorTransform` (`KismetMathLibrary.TLerp` (`self.initialLocation`) (`self.FinalLocation`) _output_get))
  (if (<= (`self.Translation`) 0.0)
    (set `self.ChangeDirection` false)))

(fn `IncrementLerp`
  ;[1 1 1] On calcule la vitesse de déplacement de l'objet suivant le framerate, la vitesse, et on la set à notre Alpha de déplacement
  (bind _output_get (set `self.Translation` (+ (`self.Translation`) (* (`self.DeltaS`) (`self.Speed`)))))
  ;[1 1 1] Après le déplacement effectif, on vérifie si on est à la fin du déplacement, et si c'est le cas on déclenche le changement de direction
  (`self.K2_SetActorTransform` (`KismetMathLibrary.TLerp` (`self.initialLocation`) (`self.FinalLocation`) _output_get))
  (if (>= (`self.Translation`) 1.0)
    (set `self.ChangeDirection` true)))

(fn `UserConstructionScript`)