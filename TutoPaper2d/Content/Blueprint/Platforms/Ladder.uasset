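; Ladder platform Blueprint that grants the player's HeroCharacter permission to climb when close to it.
; Each Tick it measures the signed X-axis offset to player 0 and sets CanClimb according to whether that lies within a narrow band around the ladder.
; Y and Z are ignored, and the flag is written every frame, both in and out of range.
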(event `self.ReceiveTick`
  (params (DeltaSeconds :type "Float (single-precision)"))
  (bind _returnvalue_x (`KismetMathLibrary.BreakVector` (`self.K2_GetActorLocation`)))
  (bind _returnvalue (`GameplayStatics.GetPlayerCharacter` 0))
  (bind _returnvalue_x_2 (`KismetMathLibrary.BreakVector` (`self.K2_GetActorLocation` (`GameplayStatics.GetPlayerCharacter` 0))))
  (`|ExecutionSequence`
    (:`then_0`
      ;[1 1 1] On calcule ici la distance entre l'échelle et nous même
      (set `self.DistanceLadder` (- _returnvalue_x _returnvalue_x_2)))
    (:`then_1`
      ;[1 1 1] Si nous sommes suffisament près de l'échelle alors nous pouvons donner l'autorisation de la monter
      (if (`KismetMathLibrary.InRange_FloatFloat` (`self.DistanceLadder`) -30.0 30.0)
        (bind _ashero_character (cast `/Game/Blueprint/Character/HeroCharacter` _returnvalue))
        (set `/Game/Blueprint/Character/HeroCharacter.CanClimb` true _ashero_character)
        (else
          (bind _ashero_character_2 (cast `/Game/Blueprint/Character/HeroCharacter` _returnvalue))
          (set `/Game/Blueprint/Character/HeroCharacter.CanClimb` false _ashero_character_2))))))

(fn `UserConstructionScript`)