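; Destructible block actor that loses health when damaged and shows its wear through a Paper2D flipbook.
; BeginPlay fills health from WallMaxHp and derives a jump rate from max health and flipbook frame count.
; Each hit subtracts truncated damage and steps the flipbook position; the jump-rate modulo only controls the FireEvents flag.
; A hit arriving when health is already zero or below destroys the actor.
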(event `self.ReceiveBeginPlay`
  (set `self.FlipbookJumpRate` (/ (`self.WallMaxHp`) (`PaperFlipbookComponent.GetFlipbookLengthInFrames` (`self.PaperFlipbook`))))
  (set `self.WallActualHp` (`self.WallMaxHp`)))

(event `self.ReceiveAnyDamage`
  (params (Damage :type "Float (single-precision)") (DamageType :type "DamageType Object Reference") (InstigatedBy :type "Controller Object Reference") (DamageCauser :type "Actor Object Reference"))
  (if (<= (`self.WallActualHp`) 0)
    (`self.K2_DestroyActor`)
    (else
      (bind _output_get (set `self.WallActualHp` (- (`self.WallActualHp`) (`KismetMathLibrary.FTrunc` Damage))))
      (`PaperFlipbookComponent.SetPlaybackPositionInFrames` (`self.PaperFlipbook`) (`self.FramePosition`) (== (mod _output_get (`self.FlipbookJumpRate`)) 0))
      (`/Engine/EditorBlueprintResources/StandardMacros.IncrementInt` (`self.FramePosition`)))))

(fn `UserConstructionScript`)